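; BP_QuestBase is a quest actor that tracks a player's progress through the staged objectives of one quest.
; It loads stages from DT_QuestData by QuestID and stores current-stage progress in a map keyed by objective ID.
; Player objective-ID events, plus BeginPlay inventory queries for one objective type, update that map.
; Completed objectives show a notification widget; finishing all advances the stage or marks the quest complete.
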(event `self.ReceiveBeginPlay`
  (`self.GetQuestDetails`)
  (add `/Game/FirstPerson/Blueprints/BP_FirstPersonCharacter.OnObjectiveIDCalled` (`/Game/FL_Common.GetMyPlayerCharacter`) (`|CreateDelegate` :!event `OnObjectiveIDHeard`))
  (for _array_element (`.Objectives_20_94F1405C45A1C211AAD81B822E5BFFF8` (break `/Game/QuestSystem/F_StageDetails` (`self.CurrentStageDetail`)))
    (bind (_objectivename _description _type _objectiveid) (break `/Game/QuestSystem/F_ObjectiveDetails` _array_element))
    (if (`|EnumEquality` _type "NewEnumerator3")
      (bind _value (`/Game/Inventory/BPC_InventorySystem.QuestQueryInventory` (`/Game/FirstPerson/Blueprints/BP_FirstPersonCharacter.BPC_InventorySystem` (`/Game/FL_Common.GetMyPlayerCharacter`)) (`KismetStringLibrary.Conv_StringToName` _objectiveid)))
      (`self.OnObjectiveIDHeard` _objectiveid _value)))
  (bind _return (`self.Are Objectives Complete`))
  (set `self.IsCompleted` _return))

(fn `Are Objectives Complete`
  (returns (Return :type Boolean))
  (locals (LocalAllComplete :type Boolean :default true))
  (for _array_element (`.Objectives_20_94F1405C45A1C211AAD81B822E5BFFF8` (break `/Game/QuestSystem/F_StageDetails` (`self.CurrentStageDetail`)))
    (bind (_objectivename _description _type _objectiveid) (break `/Game/QuestSystem/F_ObjectiveDetails` _array_element))
    (if (not (>= (`BlueprintMapLibrary.Map_Find` (`self.CurrentObjectiveProgress`) _objectiveid) (`.Quantity_14_DF652A064C89A8BDE2F597993B8397BF` (break `/Game/QuestSystem/F_ObjectiveDetails` (`self.GetObjectiveDataByID` _objectiveid)))))
      (bind _output_get (set `local.LocalAllComplete` false))
      (return _output_get)))
  (return (`local.LocalAllComplete`)))

(fn `GetObjectiveDataByID`
  (params (ObjectiveID :type String))
  (returns (`Array Element` :type "/Game/QuestSystem/F_ObjectiveDetails Structure"))
  (for _array_element (`.Objectives_20_94F1405C45A1C211AAD81B822E5BFFF8` (break `/Game/QuestSystem/F_StageDetails` (`self.CurrentStageDetail`)))
    (if (`KismetStringLibrary.EqualEqual_StrStr` ObjectiveID (`.ObjectiveID_11_2F716AB845591A5B0C29B78D8E267D28` (break `/Game/QuestSystem/F_ObjectiveDetails` _array_element)))
      (return _array_element))))

(fn `GetQuestDetails`
  (bind _currentobjectiveprogress (`self.CurrentObjectiveProgress`))
  (bind _returnvalue (`|GetDataTableRow` "/Game/QuestSystem/DT_QuestData.DT_QuestData" (`self.QuestID`))
    (:`then`
      (bind _output_get (set `self.QuestDetails` _returnvalue))
      (bind _output_get_2 (set `self.CurrentStageDetail` (`|GetArrayItem` (`.Stages_13_40F880A149C67E762B76848FF811B4FC` (break `/Game/QuestSystem/F_QuestDetails` _output_get)) (`self.CurrentStage`))))
      (`BlueprintMapLibrary.Map_Clear` _currentobjectiveprogress)
      (for _array_element (`.Objectives_20_94F1405C45A1C211AAD81B822E5BFFF8` (break `/Game/QuestSystem/F_StageDetails` _output_get_2))
        (`BlueprintMapLibrary.Map_Add` _currentobjectiveprogress (`.ObjectiveID_11_2F716AB845591A5B0C29B78D8E267D28` (break `/Game/QuestSystem/F_ObjectiveDetails` _array_element)))))))

(fn `IsObjectiveComplete`
  (params (ObjectiveID :type String))
  (bind (_questdetails_questname _questdetails_logdescription _questdetails_trackingdescription _questdetails_ismainquest _questdetails_stages) (break `/Game/QuestSystem/F_QuestDetails` (`self.QuestDetails`)))
  (bind (_objectivename _description _type _objectiveid _quantity) (break `/Game/QuestSystem/F_ObjectiveDetails` (`self.GetObjectiveDataByID` ObjectiveID)))
  (if (>= (`BlueprintMapLibrary.Map_Find` (`self.CurrentObjectiveProgress`) (`local.ObjectiveID`)) _quantity)
    (bind _returnvalue (`|CreateWidget` "/Game/QuestSystem/UI/WD_QuestNotification.WD_QuestNotification_C" null _description))
    (`UserWidget.AddToViewport` _returnvalue 0)
    (bind _return (`self.Are Objectives Complete`))
    (if _return
      (bind _result (`/Engine/EditorBlueprintResources/StandardMacros.IncrementInt` (`self.CurrentStage`))
        (:`  `
          (if (`KismetArrayLibrary.Array_IsValidIndex` _questdetails_stages _result)
            (`self.GetQuestDetails`)
            (else
              (set `self.IsCompleted` true))))))))

(fn `OnObjectiveIDHeard`
  (params (ObjectiveID :type String) (Value :type Integer :default 1))
  (bind _currentobjectiveprogress (`self.CurrentObjectiveProgress`))
  (bind (_value _returnvalue) (`BlueprintMapLibrary.Map_Find` _currentobjectiveprogress ObjectiveID))
  (if (> (`KismetMathLibrary.SignOfInteger` Value) 0)
    (if _returnvalue
      (if (< _value (`.Quantity_14_DF652A064C89A8BDE2F597993B8397BF` (break `/Game/QuestSystem/F_ObjectiveDetails` (`self.GetObjectiveDataByID` (`local.ObjectiveID`)))))
        (`BlueprintMapLibrary.Map_Add` _currentobjectiveprogress (`local.ObjectiveID`) (+ _value (`local.Value`)))
        (`self.IsObjectiveComplete` (`local.ObjectiveID`))
        (`self.OnObjectiveHeard`)
        (return))
      (else
        (return)))
    (else
      (`BlueprintMapLibrary.Map_Add` _currentobjectiveprogress (`local.ObjectiveID`) (+ (`BlueprintMapLibrary.Map_Find` _currentobjectiveprogress (`local.ObjectiveID`)) (`local.Value`)))
      (`KismetSystemLibrary.PrintString` "Hello")
      (return))))

(fn `UserConstructionScript`)