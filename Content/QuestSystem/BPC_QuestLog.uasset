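; Quest log component that records active and completed quests, handles turn-ins and drives the quest tracker widget.
; Each new quest spawns a BP_QuestBase actor, looked up by QuestID for completion and status queries.
; Turn-in adds the current stage's scaled XP reward to the player character, pops up an XP bar, then completes the quest.
; QueryCompletedQuests reports active membership and treats a missing quest actor as turned in.
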(event `self.ReceiveBeginPlay`
  (bind _asbp_first_person_character (cast `/Game/FirstPerson/Blueprints/BP_FirstPersonCharacter` (`GameplayStatics.GetPlayerCharacter` 0)))
  (set `self.PlayerCharacter` _asbp_first_person_character))

(fn `AddNewQuest`
  (params (QuestID :type Name))
  (`KismetArrayLibrary.Array_AddUnique` (`self.CurrentActiveQuest`) QuestID)
  (bind _returnvalue (`|SpawnActorFromClass` "/Game/QuestSystem/BP_QuestBase.BP_QuestBase_C" (`KismetMathLibrary.MakeTransform` (0.0 0.0 0.0)) "Undefined" "MultiplyWithRoot" null QuestID null))
  (`KismetArrayLibrary.Array_Add` (`self.CurrentQuests`) _returnvalue))

(fn `CompleteQuest`
  (params (QuestID :type Name))
  (`KismetArrayLibrary.Array_AddUnique` (`self.CompletedQuest`) QuestID)
  (`KismetArrayLibrary.Array_RemoveItem` (`self.CurrentActiveQuest`) QuestID)
  (bind _array_element (`self.GetQuestActor` QuestID))
  (set `/Game/QuestSystem/BP_QuestBase.IsTurnedIn` true _array_element)
  (`self.OnQuestCompleted` _array_element))

(fn `GetQuestActor`
  (params (QuestName :type Name))
  (returns (`Array Element` :type "/Game/QuestSystem/BP_QuestBase Object Reference"))
  (for _array_element (`self.CurrentQuests`)
    (if (== (`/Game/QuestSystem/BP_QuestBase.QuestID` _array_element) QuestName)
      (return _array_element))))

(fn `QueryActiveQuest`
  (params (QuestID :type Name))
  (returns (ReturnValue :type Boolean))
  (return (`KismetArrayLibrary.Array_Contains` (`self.CurrentActiveQuest`) QuestID)))

(fn `QueryCompletedQuests`
  (params (QuestID :type Name))
  (returns (TurnedIn :type Boolean) (ReturnValue :type Boolean))
  (bind _returnvalue (`KismetArrayLibrary.Array_Contains` (`self.CurrentActiveQuest`) QuestID))
  (bind _array_element (`self.GetQuestActor` QuestID))
  (`/Engine/EditorBlueprintResources/StandardMacros.IsValid` _array_element
    (:`Is Valid`
      (return (`/Game/QuestSystem/BP_QuestBase.IsTurnedIn` _array_element) _returnvalue))
    (:`Is Not Valid`
      (return true _returnvalue))))

(fn `TrackQuest`
  (params (QuestActor :type "/Game/QuestSystem/BP_QuestBase Object Reference"))
  (bind _tracker (`self.Tracker`)
    (:`then`
      (`/Game/QuestSystem/UI/WD_Tracker.Update` _tracker QuestActor))
    (:`else`
      (bind _returnvalue (`|CreateWidget` "/Game/QuestSystem/UI/WD_Tracker.WD_Tracker_C" null QuestActor))
      (bind _output_get (set `self.Tracker` _returnvalue))
      (`UserWidget.AddToViewport` _output_get -1))))

(fn `TurnInQuest`
  (params (QuestID :type Name))
  (bind _playercharacter (`self.PlayerCharacter`))
  (`|ExecutionSequence`
    (:`then_0`
      (bind _array_element (`self.GetQuestActor` QuestID))
      (set `/Game/FirstPerson/Blueprints/BP_FirstPersonCharacter.XP` (+ (`/Game/FirstPerson/Blueprints/BP_FirstPersonCharacter.XP` _playercharacter) (/ (`KismetMathLibrary.Conv_IntToDouble` (`.XPReward_9_AD749CAF412718E85B52AD94C0A10B14` (break `/Game/QuestSystem/F_StageDetails` (`/Game/QuestSystem/BP_QuestBase.CurrentStageDetail` _array_element)))) 100.0)) _playercharacter)
      (bind _returnvalue (`|CreateWidget` "/Game/HUD/WD_XPBar.WD_XPBar_C"))
      (`UserWidget.AddToViewport` _returnvalue 0)
      (`UserWidget.PlayAnimationForward` _returnvalue (`/Game/HUD/WD_XPBar.PopUp` _returnvalue) 1.0 false))
    (:`then_1`
      (`self.CompleteQuest` QuestID))))