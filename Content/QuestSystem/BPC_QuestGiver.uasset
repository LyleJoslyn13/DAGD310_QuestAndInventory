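; BPC_QuestGiver is a component that lets its owning actor offer a quest and its rewards to the player.
; InteractWith asks the player's quest log about the configured quest: if neither active nor completed, it shows the quest widget using data table details.
; Otherwise it shows the reward widget when the quest actor is completed but not turned in.
; Both interaction outcomes return the owner's display name.
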(fn `DisplayQuest`
  (bind (_questdata_datatable _questdata_rowname) (break `DataTableRowHandle` (`self.QuestData`)))
  (bind _returnvalue (`|GetDataTableRow` _questdata_datatable _questdata_rowname)
    (:`then`
      (bind _returnvalue_2 (`|CreateWidget` "/Game/QuestSystem/UI/WD_QuestGiver.WD_QuestGiver_C" null _returnvalue _questdata_rowname))
      (`UserWidget.AddToViewport` _returnvalue_2 0))))

(fn `DisplayRewards`
  (bind (_questdata_datatable _questdata_rowname) (break `DataTableRowHandle` (`self.QuestData`)))
  (`|GetDataTableRow` "/Game/QuestSystem/DT_QuestData.DT_QuestData" _questdata_rowname
    (:`then`
      (bind _returnvalue (`|CreateWidget` "/Game/QuestSystem/UI/WD_QuestReward.WD_QuestReward_C" null (struct) _questdata_rowname))
      (`UserWidget.AddToViewport` _returnvalue 0))))

(fn `InteractWith`
  (returns (ObjectiveID :type String))
  (bind (_questdata_datatable _questdata_rowname) (break `DataTableRowHandle` (`self.QuestData`)))
  (bind _returnvalue (`KismetSystemLibrary.GetDisplayName` (`self.GetOwner`)))
  (bind _bpc_questlog (`/Game/FirstPerson/Blueprints/BP_FirstPersonCharacter.BPC_QuestLog` (`/Game/FL_Common.GetMyPlayerCharacter`)))
  (if (and (not (`/Game/QuestSystem/BPC_QuestLog.QueryActiveQuest` _bpc_questlog _questdata_rowname)) (not (`.ReturnValue` (`/Game/QuestSystem/BPC_QuestLog.QueryCompletedQuests` _bpc_questlog _questdata_rowname))))
    (`self.DisplayQuest`)
    (return _returnvalue)
    (else
      (bind _array_element (`/Game/QuestSystem/BPC_QuestLog.GetQuestActor` _bpc_questlog _questdata_rowname))
      (if (and (`/Game/QuestSystem/BP_QuestBase.IsCompleted` _array_element) (not (`/Game/QuestSystem/BP_QuestBase.IsTurnedIn` _array_element)))
        (`self.DisplayRewards`)
        (return _returnvalue)))))